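; BP_ParentItem is the base pickup item actor, with stub data getters and an empty UseItem function.
; On overlap with a non-item actor implementing BPI_Pickupable, it sends its class, icon, stack size, colour and name through PickupItemMessage, then destroys itself.
; PushItem applies a velocity-change impulse to the mesh along the player camera's forward direction.
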(event `self.ReceiveActorBeginOverlap`
  (params (OtherActor :type "Actor Object Reference"))
  (if (`KismetSystemLibrary.DoesImplementInterface` OtherActor "/Game/GEP/Blueprints/Interfaces/BPI_Pickupable.BPI_Pickupable_C")
    (if (not (`KismetMathLibrary.ClassIsChildOf` (`GameplayStatics.GetObjectClass` OtherActor) "BP_ParentItem_C"))
      (message `/Game/GEP/Blueprints/Interfaces/BPI_Pickupable.PickupItem` OtherActor (`self.ItemClass`) (`self.ItemIcon`) (`self.StackSize`) (`self.Colour`) (`self.ItemName`))
      (`self.K2_DestroyActor`))))

(event `/Game/GEP/Blueprints/Interfaces/BPI_Pickupable.PushItem`
  (bind _returnvalue (`KismetMathLibrary.GetForwardVector` (`PlayerCameraManager.GetCameraRotation` (`GameplayStatics.GetPlayerCameraManager` 0))))
  (`PrimitiveComponent.AddVelocityChangeImpulseAtLocation` (`self.Mesh`) (* _returnvalue 250.0) (+ (* _returnvalue (15.0 0.0 0.0)) (`self.K2_GetActorLocation`)) "None"))

(fn `GetItemData`
  (returns (ItemClasss :type "Actor Class Reference") (CurrentStackAmouunt :type Integer) (MaxStackAmount :type Integer) (ItemColour :type "Color Structure") (ItemName :type String))
  (return null 0 0 (struct) ""))

(fn `GetPickupItemData`
  (returns (ItemClasss :type "Actor Class Reference") (CurrentStackAmouunt :type Integer) (MaxStackAmount :type Integer))
  (return null 0 0))

(fn `UseItem`
  (params (col :type "Color Structure"))
  (return))

(fn `UserConstructionScript`)